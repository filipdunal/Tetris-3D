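; BP_ChunkDestructed is a short-lived actor that shatters a destructible mesh as soon as it spawns.
; On BeginPlay it applies a dynamic instance of ChunkMaterial to both material slots and briefly toggles collision off and on.
; It then damages the DestructibleComponent with a strong impulse, using the actor's location as both hit point and direction.
; Collision turns off after a delay, and the actor destroys itself shortly afterwards.
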(event EventBeginPlay
  (bind _returnvalue (Transformation|GetActorLocation))
  (bind _destructiblecomponent (Variables|Default|GetDestructibleComponent))
  (bind _returnvalue_2 (Rendering|Material|CreateDynamicMaterialInstance (Variables|Default|GetChunkMaterial) "None" "None" :!class /Script/Engine.KismetMaterialLibrary))
  (bind _output_get (Variables|Default|SetMID _returnvalue_2))
  (Rendering|Material|SetMaterial _destructiblecomponent 0 _output_get)
  (Rendering|Material|SetMaterial _destructiblecomponent 1 _output_get)
  (Collision|SetActorEnableCollision false)
  (Utilities|FlowControl|Delay 0.01)
  (Collision|SetActorEnableCollision true)
  (Class|DestructibleComponent|ApplyDamage (Variables|Default|GetDestructibleComponent) 1.0 _returnvalue _returnvalue 1.5e+04)
  (Utilities|FlowControl|Delay 2.0)
  (Collision|SetActorEnableCollision false)
  (Utilities|FlowControl|Delay 3.0)
  (Actor|DestroyActor))

(event EventTick
  (params (DeltaSeconds :type Float%20%28single-precision%29)))

(fn ConstructionScript)