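; Game mode for a Tetris-style game that sets up each level, creates the HUD and starts a looping camera shake.
; Init applies the current level's tick delay and arena size from the game instance.
; Spawning feeds the play arena from a one-item random queue of allowed chunk groups, previews the next beside it, and calls game over when spawning fails.
; It also shows the game-over summary and saves level stars and points.
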(event EventBeginPlay
  (CallFunction|Init)
  ;[1 1 1] Creating HUD
  (bind _returnvalue (UserInterface|CreateWidget "/Game/Widgets/WBP_HUD.WBP_HUD_C" 0 self (.AsBP%20Tetris%20Game%20Instance (Utilities|Casting|CastToBP_TetrisGameInstance (Class|TetrisGameMode|GetTetrisGameInstance)))))
  (bind _output_get (Variables|Default|SetHudRef _returnvalue))
  (UserInterface|Viewport|AddtoViewport _output_get 0)
  (Camera|PlayWorldCameraShake "/Game/CameraShakes/BP_CameraShake_Loop.BP_CameraShake_Loop_C" "0, 0, 0" 0.0 1e+04))

(event EventTick
  (params (DeltaSeconds :type Float%20%28single-precision%29)))

(event EventSpawnNextGroupOfChunks
  ;[1 1 1] Spawning new groups of chunks
  (bind _outactors (Actor|GetAllActorsOfClass "/Game/Blueprints/BP_PlayArena.BP_PlayArena_C"))
  (for _array_element _outactors
    (bind (_spawnedgroupofchunk _success) (Default|SpawnGroupOfChunks _array_element (CallFunction|GetNextGroupOfChunksfromQueue) self))
    (Variables|Default|SetSpawned%20Group%20Of%20Chunk _spawnedgroupofchunk)
    (if (not _success)
      (Class|TetrisGameMode|GameOver)
      (else
        (CallFunction|SpawnPreviewGroupOfChunks)))))

(event EventShowSummary
  ;[1 1 1] UI Summary
  (bind _returnvalue (UserInterface|CreateWidget "/Game/Widgets/WBP_PauseMenuOld.WBP_PauseMenuOld_C" 0 true))
  (UserInterface|Viewport|AddtoViewport _returnvalue 0))

(event EventSaveProgress
  (bind _asbp_tetris_game_instance (Utilities|Casting|CastToBP_TetrisGameInstance (Game|GetGameInstance)))
  (Utilities|IsValid (Variables|/Game/Blueprints/BP_TetrisGameInstance.BP_TetrisGameInstance_C|GetTetrisSaveGame _asbp_tetris_game_instance)
    (:Is%20Valid
      (Default|SetLevelProgress (Variables|/Game/Blueprints/BP_TetrisGameInstance.BP_TetrisGameInstance_C|GetTetrisSaveGame _asbp_tetris_game_instance) (Variables|/Script/Tetris3D.TetrisGameInstance|GetCurrentLevel _asbp_tetris_game_instance) (Variables|/Script/Tetris3D.TetrisGameInstance|GetCurrentWorld _asbp_tetris_game_instance) (Class|TetrisGameMode|GetStarsReached) (Class|TetrisGameMode|GetPoints)))))

(fn ConstructionScript)

(fn Init
  (LocalVariables|SetTetrisRef (.AsBP%20Tetris%20Game%20Instance (Utilities|Casting|CastToBP_TetrisGameInstance (Class|TetrisGameMode|GetTetrisGameInstance))))
  (Variables|Default|SetGameActive true)
  (Variables|Default|SetTetrisTickDelay (.TickTime (Utilities|Struct|BreakLevelStruct (Variables|/Script/Tetris3D.TetrisGameInstance|GetCurrentLevel (LocalVariables|GetTetrisRef)))))
  (bind _outactors (Actor|GetAllActorsOfClass "/Game/Blueprints/BP_PlayArena.BP_PlayArena_C"))
  (for _array_element _outactors
    (Default|SetArenaSize _array_element (.MapWidth (Utilities|Struct|BreakLevelStruct (Variables|/Script/Tetris3D.TetrisGameInstance|GetCurrentLevel (LocalVariables|GetTetrisRef)))) (.MapDepth (Utilities|Struct|BreakLevelStruct (Variables|/Script/Tetris3D.TetrisGameInstance|GetCurrentLevel (LocalVariables|GetTetrisRef)))))))

(fn GetRandomGroupOfChunks
  (return (.AsBP%20Group%20Of%20Chunks%20Base (Utilities|Casting|CastToBP_GroupOfChunks_BaseClass (.OutItem (Utilities|Array|Random (Utilities|Struct|BreakLevelStruct (Variables|/Script/Tetris3D.TetrisGameInstance|GetCurrentLevel (.AsBP%20Tetris%20Game%20Instance (Utilities|Casting|CastToBP_TetrisGameInstance (Class|TetrisGameMode|GetTetrisGameInstance)))))))))))

(fn GetNextGroupOfChunksfromQueue
  (LocalVariables|SetToSpawn (select (Utilities|IsValidClass (Variables|Default|GetGroup%20Of%20Chunks%20In%20Queue)) (Variables|Default|GetGroup%20Of%20Chunks%20In%20Queue) (CallFunction|GetRandomGroupOfChunks)))
  (Variables|Default|SetGroup%20Of%20Chunks%20In%20Queue (CallFunction|GetRandomGroupOfChunks))
  (return (LocalVariables|GetToSpawn)))

(fn SpawnPreviewGroupOfChunks
  (Utilities|IsValid (Variables|Default|GetGroupOfChunksPreview)
    (:Is%20Valid
      (Actor|DestroyActor (Variables|Default|GetGroupOfChunksPreview)))
    (:Is%20Not%20Valid
      _))
  (bind _outactors (Actor|GetAllActorsOfClass "/Game/Blueprints/BP_PlayArena.BP_PlayArena_C"))
  (for _array_element _outactors
    (bind _returnvalue (Game|SpawnActorfromClass (Variables|Default|GetGroup%20Of%20Chunks%20In%20Queue) (Math|Transform|MakeTransform (Math|Vector|MakeVector 0.0 (+ (* (Variables|/Script/Tetris3D.PlayArena|GetWidth _array_element) 1e+02) 1e+02) 0.0)) "AlwaysSpawn" 0 0))
    (bind _output_get (Variables|Default|SetGroupOfChunksPreview _returnvalue))
    (Class|GroupOfChunks|SetPreviewMode _output_get true)))