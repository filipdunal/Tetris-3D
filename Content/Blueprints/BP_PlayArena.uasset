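; BP_PlayArena is the resizable play arena for a Tetris-style game, with a floor, four walls, bounds and a spawn point.
; SetArena rescales and repositions these parts from width and depth in grid units.
; Odd dimensions shift the spawn point and the floor's dynamic material by half a cell.
; SpawnGroupOfChunks spawns a piece at that point, failing if an overlap check finds a Chunk there.
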(event EventBeginPlay)

(event Collision|EventActorBeginOverlap
  (params (OtherActor :type Actor%20Object%20Reference)))

(event EventTick
  (params (DeltaSeconds :type Float%20%28single-precision%29)))

(event EventSetArena
  (params (NewWidth :type Integer) (NewDepth :type Integer))
  (CallFunction|SetArenaSize NewWidth NewDepth))

(fn ConstructionScript
  (bind _returnvalue (Rendering|Material|CreateDynamicMaterialInstance (Variables|Default|GetFloor) 0 "/Game/Materials/M_Floor_Inst.M_Floor_Inst" "None" :!class /Script/Engine.PrimitiveComponent))
  (Variables|Default|SetFloorMaterialInstance _returnvalue))

(fn SetArenaSize
  (params (Width :type Integer) (Depth :type Integer))
  (bind _spawnpoint (Variables|Default|GetSpawnPoint))
  (bind _spawnpoint_2 (Variables|Default|GetSpawnPoint))
  (bind _relativelocation (Variables|/Script/Engine.SceneComponent|GetRelativeLocation _spawnpoint))
  (bind _relativelocation_2 (Variables|/Script/Engine.SceneComponent|GetRelativeLocation _spawnpoint_2))
  (bind (_x _y _z) (Math|Vector|BreakVector _relativelocation_2))
  (bind (_x_2 _y_2 _z_2) (Math|Vector|BreakVector _relativelocation))
  (Variables|Default|SetWidth Width)
  (Variables|Default|SetDepth Depth)
  (Transformation|SetRelativeScale3D (Variables|Default|GetFloor) (/ (Math|Vector|MakeVector (Math|Conversions|ToFloat(Integer) Depth) (Math|Conversions|ToFloat(Integer) Width) 0.0) 1e+01))
  (Transformation|SetRelativeScale3D (Variables|Default|GetWall_1) (Math|Vector|MakeVector 1e+01 (Math|Conversions|ToFloat(Integer) Depth) 1e+01))
  (Transformation|SetRelativeScale3D (Variables|Default|GetWall_2) (Math|Vector|MakeVector (Math|Conversions|ToFloat(Integer) Width) 1e+01 1e+01))
  (Transformation|SetRelativeLocation (Variables|Default|GetWall_2) (Math|Vector|MakeVector (* (Math|Conversions|ToFloat(Integer) Depth) 5e+01) 0.0 5e+02) false true)
  (Transformation|SetRelativeLocation (Variables|Default|GetWall_4) (Math|Vector|MakeVector (* (Math|Conversions|ToFloat(Integer) Depth) -5e+01) 0.0 5e+02) false true)
  (Transformation|SetRelativeLocation (Variables|Default|GetWall_1) (Math|Vector|MakeVector 0.0 (* (Math|Conversions|ToFloat(Integer) Width) -5e+01) 5e+02) false true)
  (Transformation|SetRelativeLocation (Variables|Default|GetWall_3) (Math|Vector|MakeVector 0.0 (* (Math|Conversions|ToFloat(Integer) Width) 5e+01) 5e+02) false true)
  (Transformation|SetRelativeScale3D (Variables|Default|GetArenaBounds) (* (Math|Vector|MakeVector (Math|Conversions|ToFloat(Integer) Depth) (Math|Conversions|ToFloat(Integer) Width) 1e+01) 5e+01))
  (Utilities|FlowControl|Sequence
    (:then_0
      (if (!= (Math|Integer|%(Integer) Width 2) 0)
        (Transformation|SetRelativeLocation _spawnpoint (Math|Vector|MakeVector _x_2 5e+01 _z_2) false true)
        (Rendering|Material|SetScalarParameterValue (Variables|Default|GetFloorMaterialInstance) "WidthOffset" 5e+01 :!class /Script/Engine.MaterialInstanceDynamic)))
    (:then_1
      (if (!= (Math|Integer|%(Integer) Depth 2) 0)
        (Transformation|SetRelativeLocation _spawnpoint_2 (Math|Vector|MakeVector -5e+01 _y _z) false true)
        (Rendering|Material|SetScalarParameterValue (Variables|Default|GetFloorMaterialInstance) "DepthOffset" -5e+01 :!class /Script/Engine.MaterialInstanceDynamic)))))

(fn SpawnGroupOfChunks
  (params (GroupOfChunks :type BP%20Group%20Of%20Chunks%20Base%20Class%20Reference) (TetrisGameMode :type BP%20Tetris%20Game%20Mode%20Object%20Reference))
  (bind _returnvalue (Collision|SphereOverlapActors (Transformation|GetWorldLocation (Variables|Default|GetSpawnPoint)) 1e+02 (Utilities|Array|MakeArray "ObjectTypeQuery2") "/Script/Tetris3D.Chunk"))
  (if (not _returnvalue)
    (bind _returnvalue_2 (Game|SpawnActorfromClass GroupOfChunks (Transformation|GetWorldTransform (Variables|Default|GetSpawnPoint)) "AlwaysSpawn" 0 0))
    (return _returnvalue_2 true)
    (else
      (return 0 false))))