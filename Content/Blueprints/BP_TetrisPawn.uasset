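; BP_TetrisPawn is the player pawn for a Tetris game, acting as the camera pivot.
; Every Tick it teleports to the world origin in X and Y, setting its height as the sum of two helper functions.
; One derives height from the pawn's pitch, the other from a fifth of the Z position of the BP_TetrisGameMode's spawned chunk group, when valid.
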(event EventBeginPlay)

(event Collision|EventActorBeginOverlap
  (params (OtherActor :type Actor%20Object%20Reference)))

(event EventTick
  (params (DeltaSeconds :type Float%20%28single-precision%29))
  ;[1 1 1] Set camera center pivot based on rotation
  (Transformation|SetActorLocation (Math|Vector|MakeVector 0.0 0.0 (+ (CallFunction|GetCameraHeightBasedonRotation) (CallFunction|GetCameraHeightBasedonChunksPositions))) false true))

(fn ConstructionScript)

(fn GetCameraHeightBasedonRotation
  (return (* (- 75.0 (* (.Pitch (Math|Rotator|BreakRotator (Transformation|GetActorRotation))) -1.0)) 5.0)))

(fn GetCameraHeightBasedonChunksPositions
  (bind _asbp_tetris_game_mode (Utilities|Casting|CastToBP_TetrisGameMode (Game|GetGameMode)))
  (Utilities|IsValid (Variables|/Game/Blueprints/BP_TetrisGameMode.BP_TetrisGameMode_C|GetSpawned%20Group%20Of%20Chunk _asbp_tetris_game_mode)
    (:Is%20Valid
      (return (/ (.z (Transformation|GetActorLocation (Variables|/Game/Blueprints/BP_TetrisGameMode.BP_TetrisGameMode_C|GetSpawned%20Group%20Of%20Chunk _asbp_tetris_game_mode))) 5.0)))))