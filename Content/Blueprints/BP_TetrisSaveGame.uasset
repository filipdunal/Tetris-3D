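; Save game object for a Tetris game that stores per-level progress as an array of level save structs.
; SetLevelProgress looks up the entry matching world ID and level number through FindExistingLevelSave, then updates it or adds a new one.
; Existing entries keep the higher of old and new highscore and stars, and every call then writes the object to its save slot.
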(fn SetLevelProgress
  (params (CurrentLevel :type Level%20Struct%20Structure) (CurrentWorld :type World%20Struct%20Structure) (Stars :type Integer) (Points :type Integer))
  (Utilities|FlowControl|Sequence
    (:then_0
      (bind (_levelsave _levelsaveindex _found) (CallFunction|FindExistingLevelSave CurrentWorld CurrentLevel))
      (if _found
        (Utilities|Struct|SetmembersinLevelSaveStruct (Utilities|Array|Get(acopy) (Variables|Default|GetLevelsSave) _levelsaveindex) (Math|Integer|Max(Integer) (.Highscore (Utilities|Struct|BreakLevelSaveStruct (Utilities|Array|Get(acopy) (Variables|Default|GetLevelsSave) _levelsaveindex))) Points) (Math|Integer|Max(Integer) (.Stars (Utilities|Struct|BreakLevelSaveStruct (Utilities|Array|Get(acopy) (Variables|Default|GetLevelsSave) _levelsaveindex))) Stars))
        (else
          (Utilities|Array|Add (Variables|Default|GetLevelsSave) (Utilities|Struct|MakeLevelSaveStruct (Utilities|Struct|BreakWorldStruct CurrentWorld) (Utilities|Struct|BreakLevelStruct CurrentLevel) Points Stars)))))
    (:then_1
      (SaveGame|SaveGametoSlot self (Variables|Default|GetSaveSlotName) (Variables|Default|GetUserIndex)))))

(fn FindExistingLevelSave
  (params (CurrentWorld :type World%20Struct%20Structure) (CurrentLevel :type Level%20Struct%20Structure))
  (bind (_array_element _array_index) (Utilities|Array|ForEachLoopwithBreak (Variables|Default|GetLevelsSave) :!label _label)
    (:LoopBody
      (if (and (Utilities|Enum|Equal(Enum) (Utilities|Struct|BreakWorldStruct CurrentWorld) (.WorldID (Utilities|Struct|BreakLevelSaveStruct _array_element))) (== (.LevelNumber (Utilities|Struct|BreakLevelSaveStruct _array_element)) (Utilities|Struct|BreakLevelStruct CurrentLevel)))
        (bind _output_get (LocalVariables|SetReturnLevelSaveIndex _array_index))
        (LocalVariables|SetReturnLevelSave (Utilities|Array|Get(acopy) (Variables|Default|GetLevelsSave) _output_get))
        (LocalVariables|SetReturnFound true)
        (goto _label Break)))
    (:Completed
      (return (LocalVariables|GetReturnLevelSave) (LocalVariables|GetReturnLevelSaveIndex) (LocalVariables|GetReturnFound)))))