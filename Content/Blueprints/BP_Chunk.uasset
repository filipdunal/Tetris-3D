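; A single block of a Tetris piece that registers with the game mode's Tetris tick.
; Its visual mesh eases toward the logical mesh's transform, with an option to hold rotation, smoothing movement.
; While parented to a chunk group, a ghost mesh previews the landing spot using the group's fall distance.
; On destruction it unbinds, spawns a destructed chunk with the same material and plays a camera shake.
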(event EventBeginPlay
  (bind _astetris_game_mode (Utilities|Casting|CastToTetrisGameMode (Game|GetGameMode)))
  (EventDispatchers|BindEventtoOnTetrisTick _astetris_game_mode (EventDispatchers|CreateEvent :!event UpdateMeshTransform)))

(event EventDestroyChunk
  (bind _astetris_game_mode (Utilities|Casting|CastToTetrisGameMode (Game|GetGameMode)))
  (EventDispatchers|UnbindEventfromOnTetrisTick _astetris_game_mode (EventDispatchers|CreateEvent :!event UpdateMeshTransform))
  (Game|SpawnActorfromClass "/Game/Meshes/BP_ChunkDestructed.BP_ChunkDestructed_C" (Transformation|GetWorldTransform (Variables|Default|GetVisualMesh)) "AlwaysSpawn" 0 (Rendering|Material|GetMaterial (Variables|Default|GetVisualMesh) 0) 0)
  (Camera|PlayWorldCameraShake "/Game/CameraShakes/BP_CameraShake_Destroy.BP_CameraShake_Destroy_C" "0, 0, 0" 0.0 1e+04)
  (Actor|DestroyActor))

(event EventUpdateMeshTransform
  (params (TickTime :type Float%20%28single-precision%29))
  (Components|MoveComponentTo (Variables|Default|GetVisualMesh) (Transformation|GetWorldLocation (Variables|Character|GetMesh)) (select (Variables|Default|GetBlockUpdateMeshRotation) (Variables|/Script/Engine.SceneComponent|GetRelativeRotation (Variables|Default|GetVisualMesh)) (Transformation|GetWorldRotation (Variables|Character|GetMesh))) false false 0.09 true)
  (bind _asbp_group_of_chunks_base (Utilities|Casting|CastToBP_GroupOfChunks_Base (Actor|GetParentActor))
    (:then
      (Rendering|SetVisibility (Variables|Default|GetGhostVisualMesh) true false)
      (Transformation|SetWorldLocation (Variables|Default|GetGhostVisualMesh) (- (Transformation|GetWorldLocation (Variables|Character|GetMesh)) (Math|Vector|MakeVector 0.0 0.0 (Class|GroupOfChunks|GetFallDistance _asbp_group_of_chunks_base))) false true))
    (:CastFailed
      (Rendering|SetVisibility (Variables|Default|GetGhostVisualMesh) false false))))

(fn ConstructionScript)

(fn SetColor
  (params (New%20Material :type Material%20Interface%20Object%20Reference))
  (Rendering|Material|SetMaterial (Variables|Default|GetVisualMesh) 0 New%20Material))