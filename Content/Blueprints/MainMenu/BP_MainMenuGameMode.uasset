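; Main menu game mode for a Tetris game that prepares save data, shows the menu and launches gameplay.
; On BeginPlay it loads the save from slot, or creates a new save object if none exists, and stores it on the game instance.
; It then adds the main menu widget to the viewport and shows the mouse cursor.
; PlayLevel records the chosen level and world on the game instance before opening the main level.
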(event Custom|Play%20Level
  (params (Level :type Level%20Struct%20Structure) (World :type World%20Struct%20Structure))
  (bind _asbp_tetris_game_instance (Utilities|Casting|CastToBP_TetrisGameInstance (Game|GetGameInstance)))
  (Variables|/Script/Tetris3D.TetrisGameInstance|SetCurrentLevel _asbp_tetris_game_instance Level)
  (Variables|/Script/Tetris3D.TetrisGameInstance|SetCurrentWorld _asbp_tetris_game_instance World)
  (Game|OpenLevel(byObjectReference) "/Game/Levels/MainLevel.MainLevel"))

(event EventBeginPlay
  (Utilities|LoadGame
    (:out
      (bind _returnvalue (UserInterface|CreateWidget "/Game/Widgets/WBP_MainMenu.WBP_MainMenu_C"))
      (bind _output_get (Variables|Default|SetMainMenuWidgetRef _returnvalue))
      (UserInterface|Viewport|AddtoViewport _output_get 0)
      (Variables|/Script/Engine.PlayerController|SetbShowMouseCursor (Game|GetPlayerController 0) true))))

(event EventTick
  (params (DeltaSeconds :type Float%20%28single-precision%29)))

(fn ConstructionScript)