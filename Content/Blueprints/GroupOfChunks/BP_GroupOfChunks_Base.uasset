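; BP_GroupOfChunks_Base is a base actor for a cluster of BP_Chunk actors held as child actor components.
; On BeginPlay it picks a random material from ChunkMaterials and applies it to every chunk, so the group shares one color.
; DetachChunks replaces the group with standalone, non-floating chunks spawned at the same transforms, keeping the material and blocking mesh rotation updates, then destroys itself.
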(event EventBeginPlay
  (Variables|Default|SetCurrentChunkMaterial (.OutItem (Utilities|Array|Random (Variables|Default|GetChunkMaterials))))
  (for _array_element (Actor|GetComponentsByClass "/Script/Engine.ChildActorComponent")
    (bind _asbp_chunk (Utilities|Casting|CastToBP_Chunk (Variables|/Script/Engine.ChildActorComponent|GetChildActor _array_element)))
    (Default|SetColor _asbp_chunk (Variables|Default|GetCurrentChunkMaterial))))

(event Collision|EventActorBeginOverlap
  (params (OtherActor :type Actor%20Object%20Reference)))

(event EventTick
  (params (DeltaSeconds :type Float%20%28single-precision%29)))

(event EventDetachChunks
  (for _array_element (Actor|GetComponentsByClass "/Script/Engine.ChildActorComponent")
    (bind _asbp_chunk (Utilities|Casting|CastToBP_Chunk (Variables|/Script/Engine.ChildActorComponent|GetChildActor _array_element)))
    (bind _returnvalue (Game|SpawnActorfromClass "/Game/Blueprints/BP_Chunk.BP_Chunk_C" (Transformation|GetActorTransform _asbp_chunk) "AlwaysSpawn" 0 0))
    (Variables|/Script/Tetris3D.Chunk|SetbFloating _returnvalue false)
    (Rendering|Material|SetMaterial (Variables|/Script/Tetris3D.Chunk|GetVisualMesh _returnvalue) 0 (Variables|Default|GetCurrentChunkMaterial))
    (Variables|/Game/Blueprints/BP_Chunk.BP_Chunk_C|SetBlockUpdateMeshRotation _returnvalue true))
  (Actor|DestroyActor))

(fn ConstructionScript)